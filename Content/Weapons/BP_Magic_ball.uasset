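; BP_Magic_ball is a magic projectile weapon that sticks to what it hits and deals fixed damage.
; On a hit not matching its own Sphere, it stops movement, sets gravity scale and attaches to the hit actor in world space.
; It then disables Sphere collision, spawns an explosion emitter with the player camera's rotation and applies damage.
; The file shows no destroy call after impact.
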(event Collision|EventHit
  (params (MyComp :type Primitive%20Component%20Object%20Reference) (Other :type Actor%20Object%20Reference) (OtherComp :type Primitive%20Component%20Object%20Reference) (bSelfMoved :type Boolean) (HitLocation :type Vector :default "0, 0, 0") (HitNormal :type Vector :default "0, 0, 0") (NormalImpulse :type Vector :default "0, 0, 0") (Hit :type Hit%20Result%20Structure%20%28by%20ref%29))
  (bind _projectilemovement (Variables|Default|GetProjectileMovement))
  (bind _sphere (Variables|Collision|GetSphere))
  (if (!= Other (Variables|Collision|GetSphere))
    (Components|Movement|StopMovementImmediately _projectilemovement)
    (Variables|/Script/Engine.ProjectileMovementComponent|SetProjectileGravityScale _projectilemovement 1.0)
    (Transformation|AttachActorToActor Other "None" "KeepWorld" "KeepWorld" "KeepWorld" false)
    (Collision|SetCollisionEnabled _sphere "NoCollision")
    (Effects|SpawnEmitteratLocation "/Game/StarterContent/Particles/P_Explosion.P_Explosion" (Transformation|GetWorldLocation _sphere) (Camera|GetCameraRotation (Game|GetPlayerCameraManager 0)))
    (Game|Damage|ApplyDamage Other 15.0 0 0)))

(fn ConstructionScript)