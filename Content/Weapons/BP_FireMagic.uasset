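; BP_FireMagic is a magic weapon that plays casting animations on a modular character and sets its spell material by element.
; Mouse press plays the AM_MagicShoot montage on the character's mesh, and release plays it from the "Fire" section.
; On use, ChangeMaterial switches on the object's own name to pick the fire, water or earth entry from SpellMaterials for AttachMesh, defaulting to fire.
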(event EventOnUse
  (params (Character :type Modular%20Character%20Object%20Reference))
  (CallFunction|ChangeMaterial))

(event EventMouseButtonPressed
  (params (ModularCharacter :type Modular%20Character%20Object%20Reference) (bIsRightHand :type Boolean))
  (Animation|Montage|PlayMontage (Variables|/Script/Engine.Character|GetMesh ModularCharacter) "/Game/Animations/Fight/AnimMontages/AM_MagicShoot.AM_MagicShoot"))

(event EventMouseButtonReleased
  (params (ModularCharacter :type Modular%20Character%20Object%20Reference) (bIsRightHand :type Boolean))
  (Animation|Montage|PlayMontage (Variables|/Script/Engine.Character|GetMesh ModularCharacter) "/Game/Animations/Fight/AnimMontages/AM_MagicShoot.AM_MagicShoot" 1.0 0.0 "Fire"))

(fn ChangeMaterial
  (bind _spellmaterials (Variables|Default|GetSpellMaterials))
  (switch string (Utilities|GetObjectName self)
    (:Default
      (bind _output_get (Variables|Default|SetIndexOfMaterial 0 :!label _label))
      (Variables|/Script/Engine.SkeletalMesh|SetMaterials (Variables|Default|GetAttachMesh) (Utilities|Array|MakeArray (Utilities|Array|Get(acopy) _spellmaterials _output_get))))
    (:BP_FireMagic
      (goto _label))
    (:BP_WaterMagic
      (bind _output_get_2 (Variables|Default|SetIndexOfMaterial 1))
      (Variables|/Script/Engine.SkeletalMesh|SetMaterials (Variables|Default|GetAttachMesh) (Utilities|Array|MakeArray (Utilities|Array|Get(acopy) _spellmaterials _output_get_2))))
    (:BP_EarthMagic
      (bind _output_get_3 (Variables|Default|SetIndexOfMaterial 2))
      (Variables|/Script/Engine.SkeletalMesh|SetMaterials (Variables|Default|GetAttachMesh) (Utilities|Array|MakeArray (Utilities|Array|Get(acopy) _spellmaterials _output_get_3)))))
  (Variables|Default|SetAttachMesh (Variables|Default|GetAttachMesh)))