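; BP_Sword is a sword weapon Blueprint with the beginnings of a left-click melee combo.
; LeftMousePressed passes through a DoOnce with no reset wired, then plays a montage on the supplied mesh, using SM_ShortSword as the montage input.
; ComboCounter then increments and wraps at the length of a left, overhead and stab attack array.
; The lookup selecting an attack from that array by ComboCounter is left unconnected.
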(event EventLeftMousePressed
  (params (MeshComponent :type Skeletal%20Mesh%20Component%20Object%20Reference))
  (Utilities|FlowControl|DoOnce false
    (:Completed
      (Animation|Montage|PlayMontage MeshComponent "/Game/Animations/Fight/AnimMontages/SM_ShortSword.SM_ShortSword"
        (:then
          (bind _result (Math|Integer|IncrementInt (Variables|Default|GetComboCounter))
            (:%20%20
              (if (>= _result (Utilities|Array|Length (Utilities|Array|MakeArray "/Game/Animations/Fight/AnimMontages/AM_AttackLeft.AM_AttackLeft" "/Game/Animations/Fight/AnimMontages/AM_AttackOverhead.AM_AttackOverhead" "/Game/Animations/Fight/AnimMontages/AM_AttackStab.AM_AttackStab")))
                (Variables|Default|SetComboCounter 0)))))))))