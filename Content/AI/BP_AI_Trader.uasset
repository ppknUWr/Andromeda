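; BP_AI_Trader is an interactable trader that opens a trading UI for the player.
; Interacting creates a UI_Trader widget, passes it the trader's Inventory and Coins, adds it to the viewport, and switches player controller 0 to cursor-visible, UI-only input.
; CanBeInteractedWith always returns true and reveals the trader's Widget component as a side effect, which IsNoLongerLookedat hides again.
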(event Custom|Set%20Trader%20UI%20Variables
  (bind _ui_trader (Variables|Default|GetUI_Trader))
  (Variables|/Game/UI/UI_Trader.UI_Trader_C|SetInventory _ui_trader (Variables|Default|GetInventory))
  (Variables|/Game/UI/UI_Trader.UI_Trader_C|SetCoins _ui_trader (Variables|Default|GetCoins)))

(event EventIsNoLongerLookedat
  (params (Character :type Modular%20Character%20Object%20Reference))
  (Development|SetHiddeninGame (Variables|Default|GetWidget) true false))

(event EventInteract
  (params (Character :type Modular%20Character%20Object%20Reference))
  (bind _returnvalue (Game|GetPlayerController 0))
  (bind _returnvalue_2 (UserInterface|CreateWidget "/Game/UI/UI_Trader.UI_Trader_C" (Game|GetPlayerController 0)))
  (Variables|Default|SetUI_Trader _returnvalue_2)
  (CallFunction|SetTraderUIVariables)
  (UserInterface|Viewport|AddtoViewport _returnvalue_2 0)
  (Variables|/Script/Engine.PlayerController|SetbShowMouseCursor _returnvalue true)
  (Input|SetInputModeUIOnly _returnvalue _returnvalue_2 "DoNotLock"))

(fn ConstructionScript)

(fn CanbeInteractedwith
  (params (Character :type Modular%20Character%20Object%20Reference))
  (Development|SetHiddeninGame (Variables|Default|GetWidget) false false)
  (return true))