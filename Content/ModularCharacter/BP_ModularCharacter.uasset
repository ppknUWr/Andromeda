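; BP_ModularCharacter is a character Blueprint that sets up the player's stats and UI.
; On BeginPlay it shows a health bar HUD and loads the BasicStats row from the DT_CharacterStats data table into both current and max stats.
; Tab opens the inventory widget with the mouse cursor shown, and P opens MainUI, each switching input to UI-only.
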(event EventBeginPlay
  (bind _returnvalue (UserInterface|CreateWidget "/Game/ModularCharacter/WB_HealthBarHUD.WB_HealthBarHUD_C" (Game|GetPlayerController 0)))
  (UserInterface|Viewport|AddtoViewport _returnvalue 0)
  (bind _returnvalue_2 (Utilities|GetDataTableRow "/Game/ModularCharacter/DT_CharacterStats.DT_CharacterStats" "BasicStats")
    (:then
      (bind _output_get (Variables|Default|SetCurrentsStats _returnvalue_2))
      (Variables|Default|SetMaxStats _output_get))))

(event Input|KeyboardEvents|Tab
  (params (Key :type Key%20Structure :default "None"))
  (bind _returnvalue (Game|GetPlayerController 0))
  (:Pressed
    (bind _returnvalue_2 (UserInterface|CreateWidget "/Game/UI/UI_Inventory.UI_Inventory_C" (Game|GetPlayerController 0)))
    (UserInterface|Viewport|AddtoViewport _returnvalue_2 0)
    (Variables|/Script/Engine.PlayerController|SetbShowMouseCursor _returnvalue true)
    (Input|SetInputModeUIOnly _returnvalue _returnvalue_2 "DoNotLock")))

(event Input|KeyboardEvents|P
  (params (Key :type Key%20Structure :default "None"))
  (bind _returnvalue (Game|GetPlayerController 0))
  (:Pressed
    (bind _returnvalue_2 (UserInterface|CreateWidget "/Game/UI/MainUI.MainUI_C" _returnvalue))
    (UserInterface|Viewport|AddtoViewport _returnvalue_2 0)
    (Input|SetInputModeUIOnly _returnvalue _returnvalue_2 "DoNotLock")))

(fn ConstructionScript)