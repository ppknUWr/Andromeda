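; AI-controlled variant of the modular character that wanders at random and chases the player on sight.
; While no player is seen, Tick waits a random few seconds, then moves to a random reachable nearby point, toggling IsMoving around the move.
; Pawn sensing starts a chase toward any seen BP_ModularCharacter, and a retriggerable delay clears the sighting flag shortly after sightings stop.
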(event OnSeePawn(PawnSensing)
  (params (Pawn :type Pawn%20Object%20Reference))
  ;[1 1 1] Ai Player chase
  (bind _asbp_modular_character (Utilities|Casting|CastToBP_ModularCharacter Pawn))
  (Utilities|FlowControl|Sequence
    (:then_0
      (Variables|Default|SetPlayerInSight true)
      (AI|AIMoveTo self "0, 0, 0" _asbp_modular_character 5.0 false))
    (:then_1
      (Utilities|FlowControl|RetriggerableDelay 0.6)
      (Variables|Default|SetPlayerInSight false))))

(event EventBeginPlay)

(event Collision|EventActorBeginOverlap
  (params (OtherActor :type Actor%20Object%20Reference)))

(event EventTick
  (params (DeltaSeconds :type Float%20%28single-precision%29))
  ;[1 1 1] AI random movement
  (if (not (Variables|Default|GetPlayerInSight))
    (Utilities|FlowControl|Delay (Math|Random|RandomFloatinRange 3.0 6.0))
    (Variables|Default|SetisMoving true)
    (AI|AIMoveTo self (.RandomLocation (AI|Navigation|GetRandomReachablePointinRadius (Transformation|GetActorLocation) 8e+02 0 0)) 0 5.0 false
      (:OnSuccess
        _)
      (:OnFail
        _))
    (Variables|Default|SetisMoving false)))

(fn ConstructionScript)